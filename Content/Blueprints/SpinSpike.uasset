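; SpinSpike is a spike actor that plays a timed entrance during the game's intro.
; On BeginPlay it casts the game mode to PoundGameMode and acts only when PlayIntro is set.
; It hides the Spike component, waits on a long fixed delay, then shows it and uses MoveComponentTo to glide and rotate the root to a hard-coded transform over a few seconds.
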(event EventBeginPlay
  (bind _aspound_game_mode (Utilities|Casting|CastToPoundGameMode (Game|GetGameMode)))
  (if (Variables|/Game/Blueprints/PoundGameMode.PoundGameMode_C|GetPlayIntro _aspound_game_mode)
    (Rendering|SetVisibility (Variables|Default|GetSpike) false false)
    (Utilities|FlowControl|Delay 41.3)
    (Rendering|SetVisibility (Variables|Default|GetSpike) true false)
    (Components|MoveComponentTo (Variables|Default|GetDefaultSceneRoot) "705.000000,1671.000000,2099.000000" "0,185.000000,0.000000" false false 5.1 true)))

(fn ConstructionScript)