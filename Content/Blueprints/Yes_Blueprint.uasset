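; Clickable "Yes" actor that reloads the current level with the option `Intro=false`, likely as a restart confirmation.
; It caches the mesh's world transform at BeginPlay as the anchor for hover motion.
; Cursor hover plays the Yes sound and moves the mesh to a local Y offset from that anchor; cursor exit moves it back.
; The anchor is world-space but feeds MoveComponentTo's relative location target.
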(event MouseInput|EventActorBeginCursorOver
  (Audio|PlaySound2D "/Game/Audio/Yes.Yes")
  (Components|MoveComponentTo (Variables|Debug|GetStaticMeshComponent) (Math|Transform|TransformLocation (Variables|Default|GetStartTransform) "0,1000.000000,0.000000") "0, 0, 0" false false 0.2 false))

(event MouseInput|EventActorEndCursorOver
  (Components|MoveComponentTo (Variables|Debug|GetStaticMeshComponent) (Math|Transform|TransformLocation (Variables|Default|GetStartTransform) "0, 0, 0") "0, 0, 0" false false 0.2 false))

(event MouseInput|EventActorOnClicked
  (params (ButtonPressed :type Key%20Structure :default "AnyKey"))
  (bind _returnvalue (Game|GetCurrentLevelName true))
  (Game|OpenLevel(byName) (Utilities|String|StringToName _returnvalue) true "?Intro=false"))

(event EventBeginPlay
  (Variables|Default|SetStartTransform (Transformation|GetWorldTransform (Variables|Debug|GetStaticMeshComponent))))

(fn ConstructionScript)