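; No_Blueprint is a clickable "No" actor that quits the game when clicked.
; BeginPlay caches the static mesh's world transform as the reference for hover movement.
; Cursor-over plays the No sound and moves the mesh along that transform's Y axis, and cursor-out moves it back.
; MoveComponentTo receives these world-space points as relative location targets.
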(event MouseInput|EventActorBeginCursorOver
  (Audio|PlaySound2D "/Game/Audio/No.No")
  (Components|MoveComponentTo (Variables|Debug|GetStaticMeshComponent) (Math|Transform|TransformLocation (Variables|Default|GetStartTransform) "0,1000.000000,0.000000") "0, 0, 0" false false 0.2 false))

(event MouseInput|EventActorEndCursorOver
  (Components|MoveComponentTo (Variables|Debug|GetStaticMeshComponent) (Math|Transform|TransformLocation (Variables|Default|GetStartTransform) "0, 0, 0") "0, 0, 0" false false 0.2 false))

(event MouseInput|EventActorOnClicked
  (params (ButtonPressed :type Key%20Structure :default "AnyKey"))
  (Game|QuitGame 0 "Quit"))

(event EventBeginPlay
  (Variables|Default|SetStartTransform (Transformation|GetWorldTransform (Variables|Debug|GetStaticMeshComponent))))

(fn ConstructionScript)